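; BP_WalkingClown is a triggerable clown actor that appears, moves to a set position, then vanishes.
; The construction script gives its InterpToMovement component two relative control points, the actor's origin and the MoveToPos variable.
; ActivateEventFunction shows the TPose component and activates the movement, and the OnInterpToStop event hides TPose again when the movement stops.
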(event OnInterptoStop(InterpToMovement)
  (params (ImpactResult :type Hit%20Result%20Structure%20%28by%20ref%29) (Time :type Float%20%28single-precision%29))
  (Rendering|SetVisibility (Variables|Default|GetT-Pose) false false))

(event EventBeginPlay)

(event Collision|EventActorBeginOverlap
  (params (OtherActor :type Actor%20Object%20Reference)))

(event EventTick
  (params (DeltaSeconds :type Float%20%28single-precision%29)))

(event EventActivateEventFunction
  (Rendering|SetVisibility (Variables|Default|GetT-Pose) true false)
  (Components|Activation|Activate (Variables|Default|GetInterpToMovement) false))

(fn ConstructionScript
  (|CallParentFunction)
  (Class|InterptoMovementComponent|AddControlPointPosition (Variables|Default|GetInterpToMovement) "0, 0, 0" true)
  (Class|InterptoMovementComponent|AddControlPointPosition (Variables|Default|GetInterpToMovement) (Variables|Default|GetMoveToPos) true))