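; BP_EventManager fires a random event from its Events array when something begins overlapping its ActivationZone.
; It triggers the chosen event through an ActivateEventFunctionMessage call, then waits that event's own Delay before accepting another overlap.
; An IsReady flag, initialized in the construction script, gates re-triggering during the delay.
; Afterwards, non-repeatable events are removed from the pool, and debug strings print in either case.
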(event OnComponentBeginOverlap(ActivationZone)
  (params (OverlappedComponent :type Primitive%20Component%20Object%20Reference) (OtherActor :type Actor%20Object%20Reference) (OtherComp :type Primitive%20Component%20Object%20Reference) (OtherBodyIndex :type Integer) (bFromSweep :type Boolean) (SweepResult :type Hit%20Result%20Structure%20%28by%20ref%29))
  (if (Variables|Default|GetIsReady)
    (Variables|Default|SetIsReady false)
    (bind _output_get (Variables|Default|SetEventIndex (Math|Random|RandomInteger (Utilities|Array|Length (Variables|Default|GetEvents)))))
    (Class|BPTriggerEventInterface|ActivateEventFunction(Message) (Utilities|Array|Get(acopy) (Variables|Default|GetEvents) _output_get))
    (Utilities|FlowControl|Delay (Variables|/Game/Blueprints/BP_Event.BP_Event_C|GetDelay (Utilities|Array|Get(acopy) (Variables|Default|GetEvents) (Variables|Default|GetEventIndex))))
    (Variables|Default|SetIsReady true)
    (if (Variables|/Game/Blueprints/BP_Event.BP_Event_C|GetIsReapitable (Utilities|Array|Get(acopy) (Variables|Default|GetEvents) (Variables|Default|GetEventIndex)))
      (Development|PrintString (Utilities|String|ToString(Integer) (Variables|Default|GetEventIndex)))
      (else
        (Utilities|Array|RemoveIndex (Variables|Default|GetEvents) (Variables|Default|GetEventIndex))
        (Development|PrintString "NonReapetable")))))

(fn ConstructionScript
  (Variables|Default|SetIsReady true))