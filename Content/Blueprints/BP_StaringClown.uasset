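; BP_StaringClown is a triggered event actor that briefly reveals a clown figure under flickering light with laughter.
; Its ActivateEventFunction shows the TPose component and starts bulb and laugh audio.
; The Bulbs timeline then scales the SpotLight intensity from a LightIntensity base and hides the figure when it finishes.
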(event EventActivateEventFunction
  (Rendering|SetVisibility (Variables|Default|GetT-Pose) true false)
  (Audio|Components|Audio|Play (Variables|Default|GetBulbAudio) 0.0)
  (Audio|Components|Audio|Play (Variables|Default|GetLaughsAudio) 0.0)
  (bind _lighlevel (Timeline|Bulbs Play)
    (:Update
      (Rendering|Components|Light|SetIntensity (Variables|Default|GetSpotLight) (* (Variables|Default|GetLightIntensity) _lighlevel)))
    (:Finished
      (Rendering|SetVisibility (Variables|Default|GetT-Pose) false false))))

(fn ConstructionScript
  (|CallParentFunction))